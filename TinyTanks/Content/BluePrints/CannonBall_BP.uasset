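; Cannonball projectile actor that explodes when its collision sphere hits something, without applying damage.
; On hit it prints the struck actor's name, then spawns a small explosion effect and sound at the sphere's location.
; It destroys its mesh, collision and movement components immediately, then destroys the actor after a short delay.
; An unwired "Tank" tag check and "ENEMY HIT!" message are leftovers that never run.
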(event OnComponentHit(CollisionSphere)
  (params (HitComponent :type Primitive%20Component%20Object%20Reference) (OtherActor :type Actor%20Object%20Reference) (OtherComp :type Primitive%20Component%20Object%20Reference) (NormalImpulse :type Vector :default "0, 0, 0") (Hit :type Hit%20Result%20Structure%20%28by%20ref%29))
  (bind _collisionsphere (Variables|Default|GetCollisionSphere))
  (bind _returnvalue (Transformation|GetWorldLocation _collisionsphere))
  (Development|PrintString (Utilities|String|BuildString(Object) "" "Acertou em: " OtherActor) true true "(R=1.000000,G=0.872107,B=0.000000,A=1.000000)")
  (Effects|SpawnEmitteratLocation "/Game/StarterContent/Particles/P_SmallExplosion.P_SmallExplosion" _returnvalue)
  (Audio|PlaySoundatLocation "/Game/StarterContent/Audio/Explosion_Cue.Explosion_Cue" _returnvalue "0, 0, 0" 0.5 0.7)
  (Components|DestroyComponent (Variables|Default|Gettank_projectile_SM))
  (Components|DestroyComponent (Variables|Default|GetCollisionSphere))
  (Components|DestroyComponent (Variables|Default|GetProjectileMovement))
  (Utilities|FlowControl|Delay 3.0)
  (Actor|DestroyActor))

(fn ConstructionScript)