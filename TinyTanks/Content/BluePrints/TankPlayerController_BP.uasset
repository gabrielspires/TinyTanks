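; Player controller for a turn-based tank game in which one controller takes turns possessing each Tank_BP in the level.
; On BeginPlay it gathers all tanks into an array, possesses the one at the current index and adds the player HUD to the viewport.
; The end-turn event advances the index with wraparound, possesses that tank and resets the round timer stored on TinyTanksGameMode_BP.
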(event Custom|EndTurn_TT_Event
  ;[1 1 1] Troca de turno
  (if (== (Variables|Default|GetCurrentSelectedPlayerIndex) (- (Utilities|Array|Length (Variables|Default|GetAvailablePlayers)) 1))
    (Variables|Default|SetCurrentSelectedPlayerIndex 0)
    (else
      (bind _result (Math|Integer|IncrementInt (Variables|Default|GetCurrentSelectedPlayerIndex))
        (:%20%20
          (Variables|Default|SetCurrentSelectedPlayerIndex _result)))))
  (Pawn|Possess (Utilities|Array|Get(acopy) (Variables|Default|GetAvailablePlayers) (Variables|Default|GetCurrentSelectedPlayerIndex)))
  ;[1 1 1] Reseta o tempo do round pro proximo player
  (bind _astiny_tanks_game_mode_bp (Utilities|Casting|CastToTinyTanksGameMode_BP (Game|GetGameMode)))
  (Variables|/Game/BluePrints/TinyTanksGameMode_BP.TinyTanksGameMode_BP_C|SetCentiseconds _astiny_tanks_game_mode_bp 99)
  (Variables|/Game/BluePrints/TinyTanksGameMode_BP.TinyTanksGameMode_BP_C|SetSeconds _astiny_tanks_game_mode_bp 15))

(event EventBeginPlay
  ;[1 1 1] Procura todos os players no mapa e coloca eles em um vetor
  (bind _outactors (Actor|GetAllActorsOfClass "/Game/BluePrints/Tank_BP.Tank_BP_C"))
  (bind _output_get (Variables|Default|SetAvailablePlayers _outactors))
  (Pawn|Possess (Utilities|Array|Get(acopy) _output_get (Variables|Default|GetCurrentSelectedPlayerIndex)))
  ;[1 1 1] HUD
  (bind _returnvalue (UserInterface|CreateWidget "/Game/BluePrints/PlayerHUD_BP.PlayerHUD_BP_C"))
  (UserInterface|Viewport|AddtoViewport _returnvalue 0))

(event EventTick
  (params (DeltaSeconds :type Float%20%28single-precision%29)))

(fn ConstructionScript)