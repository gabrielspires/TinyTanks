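; Game mode for Tiny Tanks that runs a match countdown and ends the game when one or no tanks remain.
; Tick decrements centiseconds after a tiny Delay, rolling into seconds, clamping at zero and counting Tank_BP actors on each rollover.
; EndGame creates the end menu on first call, then on later calls displays it, pauses and shows the cursor.
; Pause menu logic exists but is unreachable.
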(event EventBeginPlay)

(event EventTick
  (params (DeltaSeconds :type Float%20%28single-precision%29))
  (Utilities|FlowControl|Delay 0.001)
  (Variables|Default|SetCentiseconds (- (Variables|Default|GetCentiseconds) 1))
  (if (< (Variables|Default|GetCentiseconds) 0)
    (Variables|Default|SetSeconds (- (Variables|Default|GetSeconds) 1))
    (Variables|Default|SetCentiseconds 99)
    (if (< (Variables|Default|GetSeconds) 0)
      (Variables|Default|SetSeconds 0)
      (Variables|Default|SetCentiseconds 0))
    (bind _outactors (Actor|GetAllActorsOfClass "/Game/BluePrints/Tank_BP.Tank_BP_C"))
    (if (<= (Utilities|Array|Length _outactors) 1)
      (CallFunction|EndGame))))

(fn ConstructionScript)

(fn EndGame
  (Utilities|IsValid (Variables|Default|GetEndGameMenuReference)
    (:Is%20Valid
      (Input|SetInputModeUIOnly (Game|GetPlayerController 0) (Variables|Default|GetEndGameMenuReference) "DoNotLock")
      (UserInterface|Viewport|AddtoViewport (Variables|Default|GetEndGameMenuReference) 0)
      (Game|SetGamePaused true)
      (Variables|/Script/Engine.PlayerController|SetbShowMouseCursor (Game|GetPlayerController 0) true))
    (:Is%20Not%20Valid
      (bind _returnvalue (UserInterface|CreateWidget "/Game/BluePrints/EndGameMenu_BP.EndGameMenu_BP_C"))
      (Variables|Default|SetEndGameMenuReference _returnvalue))))